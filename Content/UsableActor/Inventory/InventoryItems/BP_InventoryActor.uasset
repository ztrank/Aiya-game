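; BP_InventoryActor represents an item held in inventory, with a display name, icon texture and the class of its world pickup.
; SetValues copies the display name and class from a pickup actor.
; GetPickupActor reverses this by spawning that class at a given transform and passing itself to the pickup's SetValues.
; OnUse does nothing beyond returning true, and GetIcon returns the texture with a validity flag.
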(fn `Get Icon`
  (returns (Texture :type "Texture Object Reference") (`Has Texture` :type Boolean))
  (bind _texture (`self.Texture`))
  (return _texture (`KismetSystemLibrary.IsValid` _texture)))

(fn `Get Pickup Actor`
  (params (Character :type "/Game/FirstPersonBP/Blueprints/BP_Character Object Reference") (`Spawn Transformation` :type "Transform Structure"))
  (returns (Success :type Boolean) (`Pickup Actor` :type "/Game/UsableActor/Inventory/WorldItems/BP_PickupActor Object Reference"))
  (bind _returnvalue (`|SpawnActorFromClass` (`self.Pickup Class`) `Spawn Transformation` "Undefined" "OverrideRootScale"))
  (bind _asbp_pickup_actor (cast `/Game/UsableActor/Inventory/WorldItems/BP_PickupActor` _returnvalue)
    (:`then`
      (bind _pickup_actor (`/Game/UsableActor/Inventory/WorldItems/BP_PickupActor.Set Values` _asbp_pickup_actor self))
      (return true _pickup_actor))
    (:`CastFailed`
      (return false null))))

(fn `On Use`
  (params (Character :type "/Game/FirstPersonBP/Blueprints/BP_Character Object Reference"))
  (returns (Success :type Boolean))
  (return true))

(fn `Set Values`
  (params (`Pickup Actor` :type "/Game/UsableActor/Inventory/WorldItems/BP_PickupActor Object Reference"))
  (returns (`Inventory Actor` :type "/Game/UsableActor/Inventory/InventoryItems/BP_InventoryActor Object Reference"))
  (set `self.Display Name` (`/Game/UsableActor/Inventory/WorldItems/BP_PickupActor.Display Name` `Pickup Actor`))
  (set `self.Pickup Class` (`GameplayStatics.GetObjectClass` `Pickup Actor`))
  (return self))

(fn `UserConstructionScript`)
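; BP_PickupActor is a usable world item that gives its using character an inventory item.
; On use, it spawns its InventoryClass, casts it to BP_InventoryActor, copies values in via SetValues, passes it to the character's PickupItem, then runs the parent OnUse.
; A failed cast returns false.
; Its own SetValues does the reverse, taking display name and class from an inventory actor.
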(fn `Get Inventory Actor`
  (params (Character :type "/Game/FirstPersonBP/Blueprints/BP_Character Object Reference"))
  (returns (`Is Inventory Actor` :type Boolean) (`Inventory Actor` :type "/Game/UsableActor/Inventory/InventoryItems/BP_InventoryActor Object Reference"))
  ;[1 1 1] Create the Actor and cast as BP Inventory Actor
  (bind _returnvalue (`|SpawnActorFromClass` (`self.Inventory Class`) (`KismetMathLibrary.MakeTransform` (0.0 0.0 0.0)) "Undefined" "OverrideRootScale"))
  (bind _asbp_inventory_actor (cast `/Game/UsableActor/Inventory/InventoryItems/BP_InventoryActor` _returnvalue)
    (:`then`
      ;[1 1 1] Successful Cast, set values, return Inventory Actor and True
      (bind _inventory_actor (`/Game/UsableActor/Inventory/InventoryItems/BP_InventoryActor.Set Values` _asbp_inventory_actor self))
      (return true _inventory_actor))
    (:`CastFailed`
      ;[1 1 1] Failed Cast, return false
      (return false null))))

(fn `On Use`
  (params (Character :type "/Game/FirstPersonBP/Blueprints/BP_Character Object Reference"))
  (returns (Success :type Boolean))
  ;[1 1 1] Get The Inventory Actor Self
  (bind (_is_inventory_actor _inventory_actor) (`self.Get Inventory Actor` Character))
  (if _is_inventory_actor
    ;[1 1 1] Call pickup on the Character, and Parent on Use
    (`/Game/FirstPersonBP/Blueprints/BP_Character.PickupItem` Character _inventory_actor)
    (bind _success (`parent.On Use` Character))
    (return _success)
    (else
      (return false))))

(fn `Set Values`
  (params (`Inventory Actor` :type "/Game/UsableActor/Inventory/InventoryItems/BP_InventoryActor Object Reference"))
  (returns (`Pickup Actor` :type "/Game/UsableActor/Inventory/WorldItems/BP_PickupActor Object Reference"))
  (set `self.Display Name` (`/Game/UsableActor/Inventory/InventoryItems/BP_InventoryActor.Display Name` `Inventory Actor`))
  (set `self.Inventory Class` (`GameplayStatics.GetObjectClass` `Inventory Actor`))
  (return self))

(fn `UserConstructionScript`
  (`parent.UserConstructionScript`))